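; BP_Alien is an enemy alien that melee-attacks the player marine and can be killed by damage.
; Tick plays an attack montage when the player is in range, pausing movement until it completes; its alive check gates nothing.
; Damage lowers clamped health; at zero it disables collision, credits the marine's kill and destroys itself after a delay.
; The AIMoveTo chase loop is disconnected, and DamagePlayer is defined but not called here.
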(event `self.ReceiveBeginPlay`
  (bind _asbp_marine (cast `/Game/Blueprints/Pawns/BP_Marine` (`GameplayStatics.GetPlayerCharacter` 0)))
  (set `self.Marine` _asbp_marine))

(event `self.ReceiveTick`
  (params (DeltaSeconds :type "Float (single-precision)"))
  (`self.AlienAndMarineAreAlive`)
  (if (`self.AIShouldAttack`)
    (`self.DeactivateAIMovement`)
    (`|PlayMontage` (`self.Mesh`) "/Game/Characters/Enemy_Great_Spider/Animations/Alien_Attack1.Alien_Attack1"
      (:`OnCompleted`
        (`self.ActivateAIMovement`)))))

(event `self.ReceiveAnyDamage`
  (params (Damage :type "Float (single-precision)") (DamageType :type "DamageType Object Reference") (InstigatedBy :type "Controller Object Reference") (DamageCauser :type "Actor Object Reference"))
  (if (`self.AlienIsAlive`)
    (bind _alien_health (`self.DecreaseHealth` Damage))
    (if (== _alien_health 0.0)
      (`self.KillAI`)
      (`KismetSystemLibrary.Delay` 2.5)
      (`self.K2_DestroyActor`))))

(fn `ActivateAIMovement`
  (`ActorComponent.Activate` (`self.CharacterMovement`) false))

(fn `AIShouldAttack`
  (returns (ReturnValue :type Boolean))
  (if true
    (return (and (`self.IsWithinAttackRange`) (not (`self.IsAttacking`))))))

(fn `AlienAndMarineAreAlive`
  (if (`self.AlienIsAlive`)
    (if (`/Game/Blueprints/Pawns/BP_Marine.IsAlive` (`self.Marine`))
      _)))

(fn `AlienIsAlive`
  (returns (isAlive :type Boolean))
  (return (`self.isAlive`)))

(fn `DamagePlayer`
  (`GameplayStatics.ApplyDamage` (`GameplayStatics.GetPlayerCharacter` 0) (`self.DamagePerHit`)))

(fn `DeactivateAIMovement`
  (`ActorComponent.Deactivate` (`self.CharacterMovement`)))

(fn `DecreaseHealth`
  (params (DamageAmmount :type "Float (double-precision)"))
  (returns (`Alien Health` :type "Float (double-precision)"))
  (bind _output_get (set `self.AlienHealth` (`KismetMathLibrary.FClamp` (- (`self.AlienHealth`) DamageAmmount) 0.0 100.0)))
  (return _output_get))

(fn `IsAttacking`
  (returns (ReturnValue :type Boolean))
  (return (`AnimInstance.Montage_IsPlaying` (`SkeletalMeshComponent.GetAnimInstance` (`self.Mesh`)) null)))

(fn `IsWithinAttackRange`
  (returns (ReturnValue :type Boolean))
  (return (< (`self.GetDistanceTo` (`GameplayStatics.GetPlayerCharacter` 0)) (`self.AttackRange`))))

(fn `KillAI`
  (set `self.IsPlayerDead` true)
  (`self.DeactivateAIMovement`)
  (`self.SetActorEnableCollision` false)
  (`/Game/Blueprints/Pawns/BP_Marine.IncreaseKills` (`self.Marine`))
  (set `self.isAlive` false))

(fn `UserConstructionScript`)