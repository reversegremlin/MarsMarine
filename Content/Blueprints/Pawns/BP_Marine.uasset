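; Player Marine for a twin-stick shooter, with world-axis movement, health, death, a kill counter and a HUD widget.
; Each tick it sets control yaw from thumbstick direction or smoothed mouse-velocity direction, both deadzoned, depending on the last pressed key's device.
; Holding fire runs a looping timer of muzzle-socket line traces along control rotation that apply damage and spawn impacts, alongside muzzle flash and looped audio.
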(event `self.ReceiveAnyDamage`
  (params (Damage :type "Float (single-precision)") (DamageType :type "DamageType Object Reference") (InstigatedBy :type "Controller Object Reference") (DamageCauser :type "Actor Object Reference"))
  (if (not (`self.IsDead`))
    (bind _playerhealth (`self.DecreaseHealth` Damage))
    (if (== _playerhealth 0.0)
      (set `self.IsDead` true)
      (`self.StopFiringWeapon`)
      (`GameplayStatics.SpawnSound2D` "/Game/Sounds/173126__replix__death-sound-male.173126__replix__death-sound-male" 1.0 1.0 0.4 null))))

(event `self.ReceiveBeginPlay`
  (bind _returnvalue (`|CreateWidget` "/Game/UI/W_PlayerHUD.W_PlayerHUD_C" null self))
  (`UserWidget.AddToViewport` _returnvalue 0))

(event `Key|AnyKey`
  (params (Key :type "Key Structure"))
  (:`Pressed`
    (set `self.GamepadIsActive` (`KismetInputLibrary.Key_IsGamepadKey` Key))))

(event `InputAction|Fire Weapon`
  (params (Key :type "Key Structure"))
  (:`Pressed`
    (if (`self.IsAlive`)
      (`self.StartFiringWeapon`)
      (`self.WeaponTrace`)
      (`KismetSystemLibrary.K2_SetTimer` null "WeaponTrace" (`self.WeaponFireRate`) true)))
  (:`Released`
    (`self.StopFiringWeapon`)))

(event `self.ReceiveTick`
  (params (DeltaSeconds :type "Float (single-precision)"))
  (`self.UpdatePlayerAim`))

(event `InputAxis|Forward/Backward Axis Mapping`
  (params (AxisValue :type "Float (single-precision)"))
  (if (`self.IsAlive`)
    (`self.AddMovementInput` (1.0 0.0 0.0) AxisValue)))

(event `InputAxis|Right/Left Axis Mapping`
  (params (AxisValue :type "Float (single-precision)"))
  (if (`self.IsAlive`)
    (`self.AddMovementInput` (0.0 1.0 0.0) AxisValue)))

(fn `DecreaseHealth`
  (params (DamageAmmount :type "Float (double-precision)"))
  (returns (PlayerHealth :type "Float (double-precision)"))
  (bind _output_get (set `self.PlayerHealth` (`KismetMathLibrary.FClamp` (- (`self.PlayerHealth`) DamageAmmount) 0.0 100.0)))
  (return _output_get))

(fn `GetMouseAimDirection`
  (returns (ReturnValue :type "Rotator Structure"))
  (bind (_returnvalue_x _returnvalue_y) (`KismetMathLibrary.BreakVector2D` (`self.GetMouseVelocity`)))
  (return (`KismetMathLibrary.RInterpTo` (`Controller.GetControlRotation` (`GameplayStatics.GetPlayerController` 0)) (`KismetMathLibrary.MakeRotator` 0.0 0.0 (`KismetMathLibrary.DegAtan2` _returnvalue_x _returnvalue_y)) (`GameplayStatics.GetWorldDeltaSeconds`) (`self.MouseSmoothingStrength`))))

(fn `GetMouseVelocity`
  (returns (ReturnValue :type "Vector2D Structure"))
  (bind (_deltax _deltay) (`PlayerController.GetInputMouseDelta` (`GameplayStatics.GetPlayerController` 0)))
  (return (/ (`KismetMathLibrary.MakeVector2D` _deltax _deltay) (`GameplayStatics.GetWorldDeltaSeconds`))))

(fn `GetThumbstickAimDirection`
  (returns (ReturnValue :type "Rotator Structure"))
  (return (`KismetMathLibrary.MakeRotator` 0.0 0.0 (`KismetMathLibrary.DegAtan2` (`self.GetInputAxisValue`) (`self.GetInputAxisValue`)))))

(fn `GetWeaponTraceEndLocation`
  (returns (ReturnValue :type "Vector Structure"))
  (return (+ (`self.GetWeaponTraceStartLocation`) (* (`KismetMathLibrary.GetForwardVector` (`self.GetControlRotation`)) (`self.WeaponRange`)))))

(fn `GetWeaponTraceStartLocation`
  (returns (ReturnValue :type "Vector Structure"))
  (return (`SceneComponent.GetSocketLocation` (`self.RifleSkeletalMesh`) "MuzzleFlash")))

(fn `IncreaseKills`
  (set `self.PlayerKills` (+ (`self.PlayerKills`) 1)))

(fn `IsAlive`
  (returns (ReturnValue :type Boolean))
  (return (not (`self.IsDead`))))

(fn `IsMouseAboveDeadzone`
  (returns (ReturnValue :type Boolean))
  (return (> (`KismetMathLibrary.VSize2D` (`self.GetMouseVelocity`)) (`self.MouseDeadzone`))))

(fn `IsThumbstickAboveDeadzone`
  (returns (isInDeadzone :type Boolean))
  (return (> (`KismetMathLibrary.VSize2D` (`KismetMathLibrary.MakeVector2D` (`self.GetInputAxisValue`) (`self.GetInputAxisValue`))) (`self.ThumbstickDeadzone`))))

(fn `SpawnInpactHit`
  (params (HitLocation :type "Vector Structure"))
  (`GameplayStatics.SpawnEmitterAtLocation` "/Game/Effects/Weapons/Impacts/P_AssaultRifle_IH.P_AssaultRifle_IH" HitLocation))

(fn `StartFiringWeapon`
  (if (`self.IsAlive`)
    (`ActorComponent.Activate` (`self.P_AssaultRifle_MF`) false)
    (bind _returnvalue (`GameplayStatics.SpawnSound2D` "/Game/Sounds/Weapon_AssaultRifle/Stereo/RifleFireLoop_Cue.RifleFireLoop_Cue" 1.0 1.0 0.0 null))
    (set `self.WeaponFireSound` _returnvalue)))

(fn `StopFiringWeapon`
  (bind _weaponfiresound (`self.WeaponFireSound`))
  (`ActorComponent.Deactivate` (`self.P_AssaultRifle_MF`))
  (`/Engine/EditorBlueprintResources/StandardMacros.IsValid` _weaponfiresound
    (:`Is Valid`
      (`AudioComponent.Stop` _weaponfiresound)
      (`KismetSystemLibrary.K2_ClearTimer` null "WeaponTrace")
      (if (`self.IsAlive`)
        (`GameplayStatics.SpawnSound2D` "/Game/Sounds/Weapon_AssaultRifle/Stereo/RifleFireEnd_Cue.RifleFireEnd_Cue" 1.0 1.0 0.0 null)))))

(fn `UpdateMouseAim`
  (if (`self.IsMouseAboveDeadzone`)
    (`Controller.SetControlRotation` (`GameplayStatics.GetPlayerController` 0) (`self.GetMouseAimDirection`))))

(fn `UpdatePlayerAim`
  (if (`self.IsAlive`)
    (if (`self.GamepadIsActive`)
      (`self.UpdateThumbstickAim`)
      (else
        (`self.UpdateMouseAim`)))))

(fn `UpdateThumbstickAim`
  (if (`self.IsThumbstickAboveDeadzone`)
    (`Controller.SetControlRotation` (`GameplayStatics.GetPlayerController` 0) (`self.GetThumbstickAimDirection`))))

(fn `UserConstructionScript`)

(fn `WeaponTrace`
  (bind _outhit (`KismetSystemLibrary.LineTraceSingle` (`self.GetWeaponTraceStartLocation`) (`self.GetWeaponTraceEndLocation`) "TraceTypeQuery1"))
  (bind (_bblockinghit _binitialoverlap _time _distance _location _impactpoint _normal _impactnormal _physmat _hitactor) (`GameplayStatics.BreakHitResult` _outhit))
  (if _bblockinghit
    (`self.SpawnInpactHit` _location)
    (`GameplayStatics.ApplyDamage` _hitactor (`self.DamagePerShot`))))