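; Game mode that runs waves of alien enemies, starting the first shortly after play begins.
; SetupNewWave increments the wave and starts a looping timer that spawns aliens at random TargetPoints until AlienSpawnsRemaining reaches zero; that counter is never refilled here.
; RegisterAlienDeath removes aliens from the tracked array, prints debug messages, and starts the next wave after a delay once none remain alive or pending.
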(event `self.ReceiveBeginPlay`
  (`KismetSystemLibrary.Delay` 2.0)
  (`self.SetupNewWave`))

(event `Spawn Wave`
  (`self.SpawnAlien`))

(event `End Wave`
  (`KismetSystemLibrary.Delay` 2.0)
  (`self.SetupNewWave`))

(fn `GetRandomSpawnPoint`
  (returns (`Spawn Point` :type "TargetPoint Object Reference"))
  (bind _outactors (`GameplayStatics.GetAllActorsOfClass` "/Script/Engine.TargetPoint"))
  (return (`|GetArrayItem` _outactors (`KismetMathLibrary.RandomIntegerInRange` 0 (`KismetArrayLibrary.Array_LastIndex` _outactors)))))

(fn `IsWaveComplete`
  (returns (ReturnValue :type Boolean))
  (return (and (== (`KismetArrayLibrary.Array_Length` (`self.Aliens`)) 0) (== (`self.Alien Spawns Remaining`) 0))))

(fn `RegisterAlienDeath`
  (params (Alien :type "/Game/Blueprints/AI/BP_Alien Object Reference"))
  (bind _aliens (`self.Aliens`))
  (`KismetSystemLibrary.PrintString` (`KismetStringLibrary.Concat_StrStr` "REMOVING " (`KismetSystemLibrary.GetDisplayName` Alien)))
  (bind _returnvalue (`KismetArrayLibrary.Array_RemoveItem` _aliens Alien))
  (`KismetSystemLibrary.PrintString` (`KismetStringLibrary.Conv_BoolToString` _returnvalue))
  (`KismetSystemLibrary.PrintString` (`KismetStringLibrary.Concat_StrStr` "LENGTH NOW " (`KismetStringLibrary.Conv_IntToString` (`KismetArrayLibrary.Array_Length` _aliens))) true true (struct :`G` 0.66 :`B` 1.0 :`A` 1.0) 40.0)
  (if (`self.IsWaveComplete`)
    (`KismetSystemLibrary.PrintString` "ENDING WAVE\n")
    (`self.End Wave`)))

(fn `SetupNewWave`
  (`/Engine/EditorBlueprintResources/StandardMacros.IncrementInt` (`self.CurrentWave`)
    (:`  `
      (`KismetSystemLibrary.K2_SetTimer` null "Spawn Wave" 1.0 true))))

(fn `SpawnAlien`
  (bind _spawn_point (`self.GetRandomSpawnPoint`))
  (`/Engine/EditorBlueprintResources/StandardMacros.IsValid` _spawn_point
    (:`Is Valid`
      (bind _returnvalue (`|SpawnActorFromClass` "/Game/Blueprints/AI/BP_Alien.BP_Alien_C" (`self.GetTransform` _spawn_point) "Undefined" "OverrideRootScale" null null))
      (`/Engine/EditorBlueprintResources/StandardMacros.IsValid` _returnvalue
        (:`Is Valid`
          (`KismetArrayLibrary.Array_Add` (`self.Aliens`) _returnvalue)
          (bind _result (`/Engine/EditorBlueprintResources/StandardMacros.DecrementInt` (`self.Alien Spawns Remaining`))
            (:`  `
              (bind _output_get (set `self.Alien Spawns Remaining` _result))
              (if (== _output_get 0)
                (`KismetSystemLibrary.K2_ClearTimer` null "Spawn Wave")))))))))

(fn `UserConstructionScript`)